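; Player character with a sphere component, using Enhanced Input for control-rotation movement, look, jumping, cube spawning and shooting short-lived projectiles.
; Hits on Cube_Blueprint increment a counter whose parity swaps red and blue materials between cube and sphere.
; LoopJump only cycles and prints an enum; Jump's Completed event calls Jump again rather than StopJumping.
; Legacy axis events are empty, and the Ball movement helper functions are unused.
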(event Input|EnhancedActionEvents|EnhancedInputActionLook
  (params (ActionValue :type Vector%202D%20Structure) (ElapsedSeconds :type Float%20%28double-precision%29) (TriggeredSeconds :type Float%20%28double-precision%29) (InputAction :type Input%20Action%20Object%20Reference :default "/Game/Input/Look.Look"))
  (bind (_x _y) (Math|Vector2D|BreakVector2D ActionValue))
  ;[1 1 1] [ 캐릭터 ] 시점
  (:Triggered
    (Pawn|Input|AddControllerYawInput _x) ; "yaw"라고 검색하면 나옴(좌우)
    (Pawn|Input|AddControllerPitchInput _y) ; "pitch"라고 검색하면 나옴(상하)
  ))

(event Input|EnhancedActionEvents|EnhancedInputActionMove
  (params (ActionValue :type Vector%202D%20Structure) (ElapsedSeconds :type Float%20%28double-precision%29) (TriggeredSeconds :type Float%20%28double-precision%29) (InputAction :type Input%20Action%20Object%20Reference :default "/Game/Input/Move.Move"))
  ;[1 1 1] [ 캐릭터 ] 이동
  (:Triggered
    (Pawn|Input|AddMovementInput (Math|Vector|GetForwardVector (Math|Rotator|MakeRotator 0.0 0.0 (.yaw (Pawn|GetControlRotation :!class /Script/Engine.Pawn)))) (.y ActionValue) false) ; 직접 움직이기
    (Pawn|Input|AddMovementInput (Math|Vector|GetRightVector (Math|Rotator|MakeRotator 0.0 0.0 (.yaw (Pawn|GetControlRotation :!class /Script/Engine.Pawn)))) (.x ActionValue) false)))

(event Input|EnhancedActionEvents|EnhancedInputActionJump
  (params (ActionValue :type Boolean) (ElapsedSeconds :type Float%20%28double-precision%29) (TriggeredSeconds :type Float%20%28double-precision%29) (InputAction :type Input%20Action%20Object%20Reference :default "/Game/Input/Jump.Jump"))
  ;[1 1 1] [ 캐릭터 ] 점프
  (:Triggered
    (Character|Jump))
  (:Completed
    (Character|Jump)))

(event Input|EnhancedActionEvents|EnhancedInputActionShoot
  (params (ActionValue :type Boolean) (ElapsedSeconds :type Float%20%28double-precision%29) (TriggeredSeconds :type Float%20%28double-precision%29) (InputAction :type Input%20Action%20Object%20Reference :default "/Game/Input/Shoot.Shoot"))
  (bind _returnvalue (Transformation|GetActorTransform))
  (bind (_location _rotation) (Math|Transform|BreakTransform _returnvalue))
  ;[1 1 1] 총알
  (:Started
    (bind _returnvalue_2 (Game|SpawnActorfromClass (Variables|Default|Get총알원본) (Math|Transform|MakeTransform (+ _location (Transformation|GetActorForwardVector)) _rotation "0.500000,0.500000,0.500000") "AlwaysSpawn" 0 0))
    (AddComponent|AddProjectileMovementComponent _returnvalue_2)
    (Actor|SetLifeSpan _returnvalue_2 3.0) ; 액터가 생성된 후 남아있는 시간
  ))

(event Input|EnhancedActionEvents|EnhancedInputActionCubeSpawn
  (params (ActionValue :type Boolean) (ElapsedSeconds :type Float%20%28double-precision%29) (TriggeredSeconds :type Float%20%28double-precision%29) (InputAction :type Input%20Action%20Object%20Reference :default "/Game/Input/CubeSpawn.CubeSpawn"))
  ;[1 1 1] [ 입력액션 ] 마우스 우클릭 시 "SpawnCube" BluePrint 생성
  (:Started
    (bind _returnvalue (Game|SpawnActorfromClass (Variables|Default|Get큐브원본) (Transformation|GetActorTransform) "Undefined" 0 0))
    (bind _asspawn_cube (Utilities|Casting|CastToSpawnCube _returnvalue))
    (Transformation|SetWorldScale3D (Variables|/Game/BluePrint/SpawnCube.SpawnCube_C|GetCube _asspawn_cube) "5.000000,5.000000,5.000000")))

(event Input|EnhancedActionEvents|EnhancedInputActionLoopJump
  (params (ActionValue :type Boolean) (ElapsedSeconds :type Float%20%28double-precision%29) (TriggeredSeconds :type Float%20%28double-precision%29) (InputAction :type Input%20Action%20Object%20Reference :default "/Game/Input/LoopJump.LoopJump"))
  (:Started
    (bind _output_get (Variables|Default|Set내부열거형 (Utilities|Enum|ByteToEnumMyEnum (+ (Variables|Default|Get내부열거형) 1))))
    (if (> _output_get 5)
      (Variables|Default|Set내부열거형 "NewEnumerator10"))
    (Development|PrintString (Utilities|String|EnumtoString (Variables|Default|Get내부열거형)))))

(event EventBeginPlay
  ;[1 1 1] 키 입력 및 기본 세팅
  (bind _as플레이어_컨트롤러 (Utilities|Casting|CastToPlayerController (Pawn|GetController)))
  (Input|AddMappingContext (PlayerController|LocalPlayerSubsystems|GetEnhancedInputLocalPlayerSubsystem _as플레이어_컨트롤러) "/Game/Input/KeyMap.KeyMap" 0 "(bIgnoreAllPressedKeysUntilRelease=True,bForceImmediately=False)"))

(event Collision|EventActorBeginOverlap
  (params (OtherActor :type Actor%20Object%20Reference)))

(event EventTick
  (params (DeltaSeconds :type Float%20%28single-precision%29)))

(event Collision|EventHit
  (params (MyComp :type Primitive%20Component%20Object%20Reference) (Other :type Actor%20Object%20Reference) (OtherComp :type Primitive%20Component%20Object%20Reference) (bSelfMoved :type Boolean) (HitLocation :type Vector :default "0, 0, 0") (HitNormal :type Vector :default "0, 0, 0") (NormalImpulse :type Vector :default "0, 0, 0") (Hit :type Hit%20Result%20Structure%20%28by%20ref%29))
  (bind _sphere (Variables|Default|GetSphere))
  (bind _부딪친_횟수 (Variables|Default|Get부딪친%20횟수))
  ;[1 1 1] 충돌
  (if true
    (Development|PrintText (Utilities|Text|ToText(Boolean) (Utilities|Enum|Equal(Enum) (Utilities|GetObjectName Other) "Cube_Blueprint_C_0")))
    (bind _ascube_blueprint (Utilities|Casting|CastToCube_Blueprint Other))
    (bind _output_get (Variables|Default|SetCubeObject _ascube_blueprint))
    (Math|Integer|IncrementInt _부딪친_횟수
      (:%20%20
        (if (== (Math|Integer|%(Integer) _부딪친_횟수 2) 0)
          (Rendering|Material|SetMaterial (Variables|/Script/Engine.StaticMeshActor|GetStaticMeshComponent _output_get) 0 "/Game/Material/BlueMaterial.BlueMaterial")
          (Rendering|Material|SetMaterial _sphere 0 "/Game/Material/RedMaterial.RedMaterial")
          (else
            (Rendering|Material|SetMaterial (Variables|/Script/Engine.StaticMeshActor|GetStaticMeshComponent _output_get) 0 "/Game/Material/RedMaterial.RedMaterial")
            (Rendering|Material|SetMaterial _sphere 0 "/Game/Material/BlueMaterial.BlueMaterial")))))))

(event Input|ActionEvents|InputActionOLDINPUTJump
  (params (Key :type Key%20Structure :default "None"))
  ;[1 1 1] [ 캐릭터_구버전 ] 컨트롤러
)

(event Input|AxisEvents|InputAxisOLDINPUTTurnRight
  (params (AxisValue :type Float%20%28single-precision%29))
  ;[1 1 1] [ 캐릭터_구버전 ] 컨트롤러
)

(event Input|AxisEvents|InputAxisOLDINPUTPitchUp
  (params (AxisValue :type Float%20%28single-precision%29))
  ;[1 1 1] [ 캐릭터_구버전 ] 컨트롤러
)

(event Input|AxisEvents|InputAxisOLDINPUTMoveForward
  (params (AxisValue :type Float%20%28single-precision%29))
  ;[1 1 1] [ 캐릭터_구버전 ] 컨트롤러
)

(event Input|AxisEvents|InputAxisOLDINPUTMoveRight
  (params (AxisValue :type Float%20%28single-precision%29))
  ;[1 1 1] [ 캐릭터_구버전 ] 컨트롤러
)

(fn ConstructionScript)

(fn BallJump
  (Character|Jump)
  (return "점프가 되었습니다"))

(fn StopJump
  (Character|StopJumping))

(fn BallTurnRight
  (params (MouseX :type Float%20%28double-precision%29))
  (Pawn|Input|AddControllerYawInput MouseX)
  (return 0.0))

(fn BallPitchUp
  (params (MouseY :type Float%20%28double-precision%29))
  (Pawn|Input|AddControllerPitchInput MouseY))

(fn BallMoveForward
  (params (AxcsY :type Float%20%28double-precision%29))
  (Pawn|Input|AddMovementInput (Math|Vector|GetForwardVector (Math|Rotator|MakeRotator 0.0 0.0 (.yaw (Pawn|GetControlRotation :!class /Script/Engine.Pawn)))) AxcsY false))

(fn BallMoveRight
  (params (AxcsX :type Float%20%28double-precision%29))
  (Pawn|Input|AddMovementInput (Math|Vector|GetRightVector (Math|Rotator|MakeRotator 0.0 0.0 (.yaw (Pawn|GetControlRotation :!class /Script/Engine.Pawn)))) AxcsX false))

(fn GetEnum
  (return (Variables|Default|Get내부열거형)))