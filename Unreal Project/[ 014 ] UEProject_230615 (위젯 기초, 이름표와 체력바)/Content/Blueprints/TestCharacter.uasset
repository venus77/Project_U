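; Test player character that moves, looks, jumps and shoots through Enhanced Input, adding its mapping context on BeginPlay.
; Input events call small functions, with movement relative to control yaw.
; Shooting spawns a Bullet at the actor's transform, adds a projectile movement component at runtime and gives it a short lifespan.
; When the character itself hits a TargetCube, it swaps that cube's material.
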(event Input|EnhancedActionEvents|EnhancedInputActionInput_Move
  (params (ActionValue :type Vector%202D%20Structure) (ElapsedSeconds :type Float%20%28double-precision%29) (TriggeredSeconds :type Float%20%28double-precision%29) (InputAction :type Input%20Action%20Object%20Reference :default "/Game/Inputs/Input_Move.Input_Move"))
  (:Triggered
    (CallFunction|PlayerMove (.x ActionValue) (.y ActionValue))))

(event Input|EnhancedActionEvents|EnhancedInputActionInput_Look
  (params (ActionValue :type Vector%202D%20Structure) (ElapsedSeconds :type Float%20%28double-precision%29) (TriggeredSeconds :type Float%20%28double-precision%29) (InputAction :type Input%20Action%20Object%20Reference :default "/Game/Inputs/Input_Look.Input_Look"))
  (:Triggered
    (CallFunction|PlayerLook (.x ActionValue) (.y ActionValue))))

(event Input|EnhancedActionEvents|EnhancedInputActionInput_Jump
  (params (ActionValue :type Boolean) (ElapsedSeconds :type Float%20%28double-precision%29) (TriggeredSeconds :type Float%20%28double-precision%29) (InputAction :type Input%20Action%20Object%20Reference :default "/Game/Inputs/Input_Jump.Input_Jump"))
  (:Started
    (CallFunction|PlayerJump false))
  (:Completed
    (CallFunction|PlayerJump true)))

(event Input|EnhancedActionEvents|EnhancedInputActionInput_Shoot
  (params (ActionValue :type Boolean) (ElapsedSeconds :type Float%20%28double-precision%29) (TriggeredSeconds :type Float%20%28double-precision%29) (InputAction :type Input%20Action%20Object%20Reference :default "/Game/Inputs/Input_Shoot.Input_Shoot"))
  (:Started
    (CallFunction|PlayerShoot)))

(event EventBeginPlay
  (bind _as플레이어_컨트롤러 (Utilities|Casting|CastToPlayerController (Pawn|GetController)))
  (Utilities|IsValid (PlayerController|LocalPlayerSubsystems|GetEnhancedInputLocalPlayerSubsystem _as플레이어_컨트롤러)
    (:Is%20Valid
      (Input|AddMappingContext (PlayerController|LocalPlayerSubsystems|GetEnhancedInputLocalPlayerSubsystem _as플레이어_컨트롤러) "/Game/Inputs/_Key_Config._Key_Config" 0 "(bIgnoreAllPressedKeysUntilRelease=True,bForceImmediately=False)"))))

(event Collision|EventActorBeginOverlap
  (params (OtherActor :type Actor%20Object%20Reference)))

(event EventTick
  (params (DeltaSeconds :type Float%20%28single-precision%29)))

(event Collision|EventHit
  (params (MyComp :type Primitive%20Component%20Object%20Reference) (Other :type Actor%20Object%20Reference) (OtherComp :type Primitive%20Component%20Object%20Reference) (bSelfMoved :type Boolean) (HitLocation :type Vector :default "0, 0, 0") (HitNormal :type Vector :default "0, 0, 0") (NormalImpulse :type Vector :default "0, 0, 0") (Hit :type Hit%20Result%20Structure%20%28by%20ref%29))
  (if (== (Utilities|GetClass Other) "/Game/Blueprints/TargetCube.TargetCube_C")
    (bind _astarget_cube (Utilities|Casting|CastToTargetCube Other))
    (Rendering|Material|SetMaterial (Variables|/Game/Blueprints/TargetCube.TargetCube_C|GetCube _astarget_cube) 0 "/Engine/MaterialTemplates/VertexAnimation/AdvancedFlag.AdvancedFlag")))

(fn ConstructionScript)

(fn PlayerLook
  (params (X :type Float%20%28double-precision%29) (Y :type Float%20%28double-precision%29))
  (Pawn|Input|AddControllerYawInput X)
  (Pawn|Input|AddControllerPitchInput Y))

(fn PlayerMove
  (params (X :type Float%20%28double-precision%29) (Y :type Float%20%28double-precision%29))
  (Pawn|Input|AddMovementInput (Math|Vector|GetForwardVector (Math|Rotator|MakeRotator 0.0 0.0 (.yaw (Pawn|GetControlRotation :!class /Script/Engine.Pawn)))) Y false)
  (Pawn|Input|AddMovementInput (Math|Vector|GetRightVector (Math|Rotator|MakeRotator 0.0 0.0 (.yaw (Pawn|GetControlRotation :!class /Script/Engine.Pawn)))) X false))

(fn PlayerJump
  (params (StopAction :type Boolean))
  (if StopAction
    (Character|StopJumping)
    (else
      (Character|Jump))))

(fn PlayerShoot
  (bind _returnvalue (Transformation|GetActorTransform))
  (bind _returnvalue_2 (Game|SpawnActorfromClass (Variables|Default|GetBullet) (Math|Transform|MakeTransform (.location _returnvalue) (.rotation _returnvalue) "1.000000,1.000000,1.000000") "Undefined" self 0))
  (AddComponent|AddProjectileMovementComponent _returnvalue_2)
  (Actor|SetLifeSpan _returnvalue_2 5.0))