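; Bullet_2 is a projectile actor that pushes TargetCube actors it hits and shows a splash effect.
; BeginPlay adds its ProjectileMovement component at runtime and gives the bullet a short lifespan.
; On Hit against that exact class, it applies the hit normal as an impulse at the impact point and spawns a pooled particle system along the surface normal.
; Unconnected nodes keep alternative impulse and effect-actor approaches.
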(event EventBeginPlay
  ;[1 1 1] 컴포넌트 직접 작성의 경우
  (AddComponent|AddProjectileMovementComponent)
  (Actor|SetLifeSpan 5.0))

(event Collision|EventActorBeginOverlap
  (params (OtherActor :type Actor%20Object%20Reference)))

(event EventTick
  (params (DeltaSeconds :type Float%20%28single-precision%29)))

(event Collision|EventHit
  (params (MyComp :type Primitive%20Component%20Object%20Reference) (Other :type Actor%20Object%20Reference) (OtherComp :type Primitive%20Component%20Object%20Reference) (bSelfMoved :type Boolean) (HitLocation :type Vector :default "0, 0, 0") (HitNormal :type Vector :default "0, 0, 0") (NormalImpulse :type Vector :default "0, 0, 0") (Hit :type Hit%20Result%20Structure%20%28by%20ref%29))
  (bind (_bblockinghit _binitialoverlap _time _distance _location _impactpoint _normal _impactnormal) (Collision|BreakHitResult Hit))
  (if (== (Utilities|GetClass Other) "/Game/Blueprints/TargetCube.TargetCube_C")
    (bind _astarget_cube (Utilities|Casting|CastToTargetCube Other))
    ;[1 0 0.04904] 부딪친 곳에 집중해서 힘을 줄 경우
    (Physics|AddImpulseatLocation (Variables|/Game/Blueprints/TargetCube.TargetCube_C|GetCube _astarget_cube) HitNormal HitLocation "None")
    (Niagara|SpawnSystematLocation "/Game/FX/Niagara/Particle_Splash.Particle_Splash" _location (Math|Conversions|RotationFromXVector _impactnormal) "1.000000,1.000000,1.000000" true true "AutoRelease")))

(fn ConstructionScript)