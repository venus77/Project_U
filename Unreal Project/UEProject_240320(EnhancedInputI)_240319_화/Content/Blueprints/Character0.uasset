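; Player-controlled Character Blueprint that provides basic movement, camera look and jumping through Enhanced Input.
; BeginPlay adds the KeyMap mapping context to the owning player controller's input subsystem.
; Move input follows the control rotation's yaw, Look drives controller yaw and pitch, and Jump starts and stops the built-in jump.
; Hit events print a Korean collision message, while overlap and Tick are empty.
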(event Input|EnhancedActionEvents|EnhancedInputActionLook
  (params (ActionValue :type Vector%202D%20Structure) (ElapsedSeconds :type Float%20%28double-precision%29) (TriggeredSeconds :type Float%20%28double-precision%29) (InputAction :type Input%20Action%20Object%20Reference :default "/Game/Inputs/Look.Look"))
  (bind (_x _y) (Math|Vector2D|BreakVector2D ActionValue))
  (:Triggered
    (Pawn|Input|AddControllerYawInput _x)
    (Pawn|Input|AddControllerPitchInput _y)))

(event Input|EnhancedActionEvents|EnhancedInputActionMove
  (params (ActionValue :type Vector%202D%20Structure) (ElapsedSeconds :type Float%20%28double-precision%29) (TriggeredSeconds :type Float%20%28double-precision%29) (InputAction :type Input%20Action%20Object%20Reference :default "/Game/Inputs/Move.Move"))
  (:Triggered
    (Pawn|Input|AddMovementInput (Math|Vector|GetForwardVector (Math|Rotator|MakeRotator 0.0 0.0 (.yaw (Pawn|GetControlRotation :!class /Script/Engine.Pawn)))) (.y ActionValue) false)
    (Pawn|Input|AddMovementInput (Math|Vector|GetRightVector (Math|Rotator|MakeRotator 0.0 0.0 (.yaw (Pawn|GetControlRotation :!class /Script/Engine.Pawn)))) (.x ActionValue) false)))

(event Input|EnhancedActionEvents|EnhancedInputActionJump
  (params (ActionValue :type Boolean) (ElapsedSeconds :type Float%20%28double-precision%29) (TriggeredSeconds :type Float%20%28double-precision%29) (InputAction :type Input%20Action%20Object%20Reference :default "/Game/Inputs/Jump.Jump"))
  (:Triggered
    (Character|Jump))
  (:Completed
    (Character|StopJumping)))

(event EventBeginPlay
  (bind _as플레이어_컨트롤러 (Utilities|Casting|CastToPlayerController (Pawn|GetController)))
  (Input|AddMappingContext (PlayerController|LocalPlayerSubsystems|GetEnhancedInputLocalPlayerSubsystem _as플레이어_컨트롤러) "/Game/Inputs/KeyMap.KeyMap" 0 "(bIgnoreAllPressedKeysUntilRelease=True,bForceImmediately=False)"))

(event Collision|EventActorBeginOverlap
  (params (OtherActor :type Actor%20Object%20Reference)))

(event EventTick
  (params (DeltaSeconds :type Float%20%28single-precision%29)))

(event Collision|EventHit
  (params (MyComp :type Primitive%20Component%20Object%20Reference) (Other :type Actor%20Object%20Reference) (OtherComp :type Primitive%20Component%20Object%20Reference) (bSelfMoved :type Boolean) (HitLocation :type Vector :default "0, 0, 0") (HitNormal :type Vector :default "0, 0, 0") (NormalImpulse :type Vector :default "0, 0, 0") (Hit :type Hit%20Result%20Structure%20%28by%20ref%29))
  (Development|PrintText "부딪쳤습니다."))

(fn ConstructionScript)