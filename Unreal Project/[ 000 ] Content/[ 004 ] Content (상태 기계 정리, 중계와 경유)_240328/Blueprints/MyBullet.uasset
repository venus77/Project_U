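; MyBullet is a physics-driven bullet actor that knocks cube targets when it hits them.
; Its Fire function applies a force from the supplied direction vector, while projectile-movement and impulse alternatives sit unconnected.
; On Hit, it matches the other actor's display name to Cube_Blueprint, casts it, applies the unscaled hit normal as an impulse at the hit location, then destroys itself.
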(event EventBeginPlay)

(event EventTick
  (params (DeltaSeconds :type Float%20%28single-precision%29)))

(event Collision|EventHit
  (params (MyComp :type Primitive%20Component%20Object%20Reference) (Other :type Actor%20Object%20Reference) (OtherComp :type Primitive%20Component%20Object%20Reference) (bSelfMoved :type Boolean) (HitLocation :type Vector :default "0, 0, 0") (HitNormal :type Vector :default "0, 0, 0") (NormalImpulse :type Vector :default "0, 0, 0") (Hit :type Hit%20Result%20Structure%20%28by%20ref%29))
  (if (Utilities|Enum|Equal(Enum) (Utilities|GetDisplayName Other) "Cube_Blueprint")
    (bind _ascube_blueprint (Utilities|Casting|CastToCube_Blueprint Other))
    (Physics|AddImpulseatLocation (Variables|/Script/Engine.StaticMeshActor|GetStaticMeshComponent _ascube_blueprint) HitNormal HitLocation "None")
    (Actor|DestroyActor)))

(fn ConstructionScript)

(fn Fire
  (params (Direction :type Vector))
  (bind (_x _y _z) (Math|Vector|BreakVector Direction))
  (Physics|AddForce :Force (Math|Vector|MakeVector _x _y _z)) ; 연속되는 힘
)