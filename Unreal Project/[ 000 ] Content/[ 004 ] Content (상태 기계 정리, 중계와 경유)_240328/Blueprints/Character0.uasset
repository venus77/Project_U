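; Player character with a sphere mesh that moves, looks and jumps through Enhanced Input, using a mapping context added on BeginPlay.
; Input actions also spawn bullets with a runtime-added projectile movement component, spawn scaled cubes, cycle an enum, and set a force-jump flag; getters expose both values.
; Hitting one named cube increments a counter whose parity swaps materials between cube and sphere.
; Legacy axis events are empty, and their Ball* helper functions are disconnected.
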(event Input|EnhancedActionEvents|EnhancedInputActionLook
  (params (ActionValue :type Vector%202D%20Structure) (ElapsedSeconds :type Float%20%28double-precision%29) (TriggeredSeconds :type Float%20%28double-precision%29) (InputAction :type Input%20Action%20Object%20Reference :default "/Game/Inputs/Look.Look"))
  (bind (_x _y) (Math|Vector2D|BreakVector2D ActionValue))
  (:Triggered
    (Pawn|Input|AddControllerYawInput _x)
    (Pawn|Input|AddControllerPitchInput _y)))

(event Input|EnhancedActionEvents|EnhancedInputActionMove
  (params (ActionValue :type Vector%202D%20Structure) (ElapsedSeconds :type Float%20%28double-precision%29) (TriggeredSeconds :type Float%20%28double-precision%29) (InputAction :type Input%20Action%20Object%20Reference :default "/Game/Inputs/Move.Move"))
  (:Triggered
    (Pawn|Input|AddMovementInput (Math|Vector|GetForwardVector (Math|Rotator|MakeRotator 0.0 0.0 (.yaw (Pawn|GetControlRotation :!class /Script/Engine.Pawn)))) (.y ActionValue) false)
    (Pawn|Input|AddMovementInput (Math|Vector|GetRightVector (Math|Rotator|MakeRotator 0.0 0.0 (.yaw (Pawn|GetControlRotation :!class /Script/Engine.Pawn)))) (.x ActionValue) false)))

(event Input|EnhancedActionEvents|EnhancedInputActionJump
  (params (ActionValue :type Boolean) (ElapsedSeconds :type Float%20%28double-precision%29) (TriggeredSeconds :type Float%20%28double-precision%29) (InputAction :type Input%20Action%20Object%20Reference :default "/Game/Inputs/Jump.Jump"))
  (:Triggered
    (Character|Jump))
  (:Completed
    (Character|StopJumping)))

(event Input|EnhancedActionEvents|EnhancedInputActionShoot
  (params (ActionValue :type Boolean) (ElapsedSeconds :type Float%20%28double-precision%29) (TriggeredSeconds :type Float%20%28double-precision%29) (InputAction :type Input%20Action%20Object%20Reference :default "/Game/Inputs/Shoot.Shoot"))
  (bind _returnvalue (Transformation|GetActorTransform))
  (bind (_location _rotation) (Math|Transform|BreakTransform _returnvalue))
  (:Started
    (bind _returnvalue_2 (Game|SpawnActorfromClass (Variables|Default|Get총알원본) (Math|Transform|MakeTransform (+ _location (Transformation|GetActorForwardVector)) _rotation "0.500000,0.500000,0.500000") "AlwaysSpawn" 0 0))
    (AddComponent|AddProjectileMovementComponent _returnvalue_2)
    (Actor|SetLifeSpan _returnvalue_2 5.0)))

(event Input|EnhancedActionEvents|EnhancedInputActionCubeSpawn
  (params (ActionValue :type Boolean) (ElapsedSeconds :type Float%20%28double-precision%29) (TriggeredSeconds :type Float%20%28double-precision%29) (InputAction :type Input%20Action%20Object%20Reference :default "/Game/Inputs/CubeSpawn.CubeSpawn"))
  (:Started
    (bind _returnvalue (Game|SpawnActorfromClass (Variables|Default|Get큐브원본) (Transformation|GetActorTransform) "Undefined" 0 0))
    (bind _asspawn_cube (Utilities|Casting|CastToSpawnCube _returnvalue))
    (Transformation|SetWorldScale3D (Variables|/Game/Blueprints/SpawnCube.SpawnCube_C|GetCube _asspawn_cube) "5.000000,5.000000,5.000000")))

(event Input|EnhancedActionEvents|EnhancedInputActionLoopEnum
  (params (ActionValue :type Boolean) (ElapsedSeconds :type Float%20%28double-precision%29) (TriggeredSeconds :type Float%20%28double-precision%29) (InputAction :type Input%20Action%20Object%20Reference :default "/Game/Inputs/LoopEnum.LoopEnum"))
  (:Started
    (bind _output_get (Variables|Default|Set내부열거형 (Utilities|Enum|ByteToEnumMyEnum (+ (Variables|Default|Get내부열거형) 1))))
    (if (> _output_get 5)
      (Variables|Default|Set내부열거형 "NewEnumerator8"))
    (Development|PrintString (Utilities|String|EnumtoString (Variables|Default|Get내부열거형)))))

(event Input|EnhancedActionEvents|EnhancedInputActionForceJump
  (params (ActionValue :type Boolean) (ElapsedSeconds :type Float%20%28double-precision%29) (TriggeredSeconds :type Float%20%28double-precision%29) (InputAction :type Input%20Action%20Object%20Reference :default "/Game/Inputs/ForceJump.ForceJump"))
  (:Started
    (Variables|Default|Set짬프 true)))

(event EventBeginPlay
  (bind _as플레이어_컨트롤러 (Utilities|Casting|CastToPlayerController (Pawn|GetController)))
  (Input|AddMappingContext (PlayerController|LocalPlayerSubsystems|GetEnhancedInputLocalPlayerSubsystem _as플레이어_컨트롤러) "/Game/Inputs/KeyMap.KeyMap" 0 "(bIgnoreAllPressedKeysUntilRelease=True,bForceImmediately=False)"))

(event Collision|EventActorBeginOverlap
  (params (OtherActor :type Actor%20Object%20Reference)))

(event EventTick
  (params (DeltaSeconds :type Float%20%28single-precision%29)))

(event Collision|EventHit
  (params (MyComp :type Primitive%20Component%20Object%20Reference) (Other :type Actor%20Object%20Reference) (OtherComp :type Primitive%20Component%20Object%20Reference) (bSelfMoved :type Boolean) (HitLocation :type Vector :default "0, 0, 0") (HitNormal :type Vector :default "0, 0, 0") (NormalImpulse :type Vector :default "0, 0, 0") (Hit :type Hit%20Result%20Structure%20%28by%20ref%29))
  (bind _sphere (Variables|Default|GetSphere))
  (bind _부딪친_횟수 (Variables|Default|Get부딪친%20횟수))
  (if (Utilities|Enum|Equal(Enum) (Utilities|GetObjectName Other) "Cube_Blueprint_C_0")
    (Development|PrintText "부딪쳤습니다.")
    (bind _ascube_blueprint (Utilities|Casting|CastToCube_Blueprint Other))
    (bind _output_get (Variables|Default|SetCubeObject _ascube_blueprint))
    (Math|Integer|IncrementInt _부딪친_횟수
      (:%20%20
        (if (== (Math|Integer|%(Integer) _부딪친_횟수 2) 0)
          (Rendering|Material|SetMaterial (Variables|/Script/Engine.StaticMeshActor|GetStaticMeshComponent _output_get) 0 "/Game/Blueprints/BlueMaterial.BlueMaterial")
          (Rendering|Material|SetMaterial _sphere 0 "/Game/Blueprints/MyMaterial.MyMaterial")
          (else
            (Rendering|Material|SetMaterial (Variables|/Script/Engine.StaticMeshActor|GetStaticMeshComponent _output_get) 0 "/Game/Blueprints/MyMaterial.MyMaterial")
            (Rendering|Material|SetMaterial _sphere 0 "/Game/Blueprints/BlueMaterial.BlueMaterial")))))))

(event Input|ActionEvents|InputActionOLDINPUT_Jump
  (params (Key :type Key%20Structure :default "None")))

(event Input|AxisEvents|InputAxisOLDINPUT_TurnRight
  (params (AxisValue :type Float%20%28single-precision%29)))

(event Input|AxisEvents|InputAxisOLDINPUT_PitchUp
  (params (AxisValue :type Float%20%28single-precision%29)))

(event Input|AxisEvents|InputAxisOLDINPUT_MoveForward
  (params (AxisValue :type Float%20%28single-precision%29)))

(event Input|AxisEvents|InputAxisOLDINPUT_MoveRight
  (params (AxisValue :type Float%20%28single-precision%29)))

(fn ConstructionScript)

(fn BallJump
  (Character|Jump)
  (return "점프가 되었습니다!"))

(fn StopJump
  (Character|StopJumping))

(fn BallTurnRight
  (params (MouseX :type Float%20%28double-precision%29))
  (Pawn|Input|AddControllerYawInput MouseX)
  (return MouseX))

(fn BallPitchUp
  (params (MouseY :type Float%20%28double-precision%29))
  (Pawn|Input|AddControllerPitchInput MouseY))

(fn BallMoveForward
  (params (AxisY :type Float%20%28double-precision%29))
  (Pawn|Input|AddMovementInput (Math|Vector|GetForwardVector (Math|Rotator|MakeRotator 0.0 0.0 (.yaw (Pawn|GetControlRotation :!class /Script/Engine.Pawn)))) AxisY false))

(fn BallMoveRight
  (params (AxisX :type Float%20%28double-precision%29))
  (Pawn|Input|AddMovementInput (Math|Vector|GetRightVector (Math|Rotator|MakeRotator 0.0 0.0 (.yaw (Pawn|GetControlRotation :!class /Script/Engine.Pawn)))) AxisX false))

(fn GetEnum
  (return (Variables|Default|Get내부열거형)))

(fn GetJamp
  (return (Variables|Default|Get짬프)))