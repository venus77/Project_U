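; TargetCube is a target actor that detects hits from a TestCharacter or Bullet.
; A qualifying Hit calls MoveUp with Enable off, so the upward impulse it would apply to the Cube never fires.
; CountAndDestroy, which prints a hit count and destroys the actor at five, is left unwired alongside other disconnected movement experiments and a Picking flag.
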(event EventBeginPlay)

(event Collision|EventActorBeginOverlap
  (params (OtherActor :type Actor%20Object%20Reference)))

(event EventTick
  (params (DeltaSeconds :type Float%20%28single-precision%29)))

(event Collision|EventHit
  (params (MyComp :type Primitive%20Component%20Object%20Reference) (Other :type Actor%20Object%20Reference) (OtherComp :type Primitive%20Component%20Object%20Reference) (bSelfMoved :type Boolean) (HitLocation :type Vector :default "0, 0, 0") (HitNormal :type Vector :default "0, 0, 0") (NormalImpulse :type Vector :default "0, 0, 0") (Hit :type Hit%20Result%20Structure%20%28by%20ref%29))
  (bind _returnvalue (Utilities|GetClass Other))
  (if (or (== _returnvalue "/Game/Blueprints/TestCharacter.TestCharacter_C") (== _returnvalue "/Game/Blueprints/Bullet.Bullet_C"))
    (Utilities|FlowControl|Sequence
      (:then_0
        (CallFunction|MoveUp false)))))

(fn ConstructionScript)

(fn CountandDestroy
  (bind _result (Math|Integer|IncrementInt (Variables|Default|GetHitCount))
    (:%20%20
      (Development|PrintString (Utilities|String|ToString(Integer) _result))
      (if (== _result 5)
        (Actor|DestroyActor)))))

(fn MoveUp
  (params (Enable :type Boolean))
  (if Enable
    (Physics|AddImpulse (Variables|Default|GetCube) (* (Math|Vector|GetUpVector (.rotation (Transformation|GetActorTransform))) 1e+06) "None" false)))