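; BP_NZombie is a zombie actor Blueprint holding basic health state and a routine for spawning more zombies.
; ResetHp restores CurHp to MaxHp, and IsDead sets and returns IsDie based on CurHp being exactly zero.
; SpawnZombie loops up to MaxZombieCount spawning copies of its own class with collision adjustment, without a computed location.
; The event graph and construction script are empty, and nothing here calls these functions.
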(event EventBeginPlay)

(event Collision|EventActorBeginOverlap
  (params (OtherActor :type Actor%20Object%20Reference)))

(event EventTick
  (params (DeltaSeconds :type Float%20%28single-precision%29)))

(fn ConstructionScript)

(fn ResetHp
  (Variables|Default|SetCur_Hp (Variables|Default|GetMax_Hp)))

(fn IsDead
  (if (== (Variables|Default|GetCur_Hp) 0.0)
    (bind _output_get (Variables|Default|SetIs_Die true))
    (return _output_get)
    (else
      (bind _output_get_2 (Variables|Default|SetIs_Die false))
      (return _output_get_2))))

(fn SpawnZombie
  (for _index (range 0 (Variables|Default|GetMax_Zombie_Count))
    (Game|SpawnActorfromClass "BP_NZombie_C" (Math|Transform|MakeTransform "0, 0, 0" "0, 0, 0" "1.000000,1.000000,1.000000") "AdjustIfPossibleButAlwaysSpawn" 0 0)))