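; Zombie character Blueprint that handles damage, death and attack state, and bridges AI state to its animation.
; Damage goes through StatComponents: a true result triggers the death animation, disables capsule collision and destroys the actor after a delay, otherwise a random hit montage plays.
; Helper functions copy sight and range Blackboard flags into ABP_Zombie and expose an attack flag that stops movement when set.
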(event EventBeginPlay
  (bind _asabp_zombie (Utilities|Casting|CastToABP_Zombie (Components|SkeletalMesh|GetAnimInstance (Variables|Character|GetMesh))))
  (Variables|Default|SetAnim _asabp_zombie))

(event Collision|EventActorBeginOverlap
  (params (OtherActor :type Actor%20Object%20Reference)))

(event EventTick
  (params (DeltaSeconds :type Float%20%28single-precision%29)))

(event Game|Damage|EventAnyDamage
  (params (Damage :type Float%20%28single-precision%29) (DamageType :type Damage%20Type%20Object%20Reference) (InstigatedBy :type Controller%20Object%20Reference) (DamageCauser :type Actor%20Object%20Reference))
  (Variables|Default|SetDamage%20Causer DamageCauser)
  (bind _is_dead (Default|DecreaseHealth (Variables|Default|GetStatComponents) Damage))
  (bind _output_get (Variables|Default|SetIsHit _is_dead))
  (if _output_get
    (Default|SetZombieIsDead (Variables|Default|GetAnim))
    (Collision|SetCollisionEnabled (Variables|Collision|GetCapsuleComponent) "NoCollision")
    (Utilities|FlowControl|Delay 5.0)
    (Actor|DestroyActor)
    (Development|PrintString "Hello")
    (else
      (CallFunction|PlayHitAnim (Variables|Default|GetHitAnim)))))

(fn ConstructionScript)

(fn SetIsSight
  (Utilities|IsValid (Variables|Character|GetMesh)
    (:Is%20Valid
      (Variables|/Game/Character/ABP_Zombie.ABP_Zombie_C|SetIsSight (Variables|Default|GetAnim) (ScalableFloat|GetValueasBool (Variables|Default|GetBlackboard) (Variables|Default|GetIsSIght))))))

(fn SetIsRange
  (Utilities|IsValid (Variables|Character|GetMesh)
    (:Is%20Valid
      (Variables|/Game/Character/ABP_Zombie.ABP_Zombie_C|SetIsRange (Variables|Default|GetAnim) (ScalableFloat|GetValueasBool (Variables|Default|GetBlackboard) (Variables|Default|GetIsRange))))))

(fn GetAttack
  (return (Variables|Default|GetShouldAttack)))

(fn SetAttack
  (params (StartAttack :type Boolean))
  (Utilities|FlowControl|Sequence
    (:then_0
      (Variables|Default|SetShouldAttack StartAttack))
    (:then_1
      (if StartAttack
        (Components|Movement|StopMovementImmediately (Variables|Character|GetCharacterMovement))))))

(fn PlayHitAnim
  (params (HitAnim :type Array%20of%20Anim%20Montage%20Object%20References))
  (Animation|PlayAnimMontage (Utilities|Array|Get(acopy) HitAnim (Math|Random|RandomIntegerinRange 0 (- (Utilities|Array|Length HitAnim) 1))) 1.0 "None"))